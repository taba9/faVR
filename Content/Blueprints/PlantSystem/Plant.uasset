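; Spline-based plant actor that grows taller each time Interact is called, until its random growth progress reaches full.
; The construction script builds spline meshes along MainSpline, with an optional root mesh and a head mesh at the tip.
; Interact adds one extra point and segment only once, then raises points with random sideways jitter, refits the meshes and moves the head.
; The leaf-spawning logic is present but never runs.
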(event `/Game/Blueprints/InteractionInterface.Interact`
  (bind _growingrandomxz (`self.GrowingRandomXZ`))
  (bind _mainspline (`self.MainSpline`))
  (bind _mainspline_2 (`self.MainSpline`))
  (bind _returnvalue (`SplineComponent.GetNumberOfSplinePoints` (`self.MainSpline`)))
  (bind _returnvalue_2 (`SplineComponent.GetNumberOfSplinePoints` _mainspline))
  (bind _returnvalue_3 (* _growingrandomxz -1.0))
  (bind _output_get (set `self.GrowProgress` (`KismetMathLibrary.FClamp` (+ (`self.GrowProgress`) (`KismetMathLibrary.RandomFloatInRange` 0.0 (`self.GrowStep`))) 0.0 1.0)))
  (if (< _output_get 1.0)
    (set `self.HeightToGrow` (* (`self.EstimatedMaxHeight`) (`self.GrowStep`)))
    (if (>= (`self.GrowProgress`) -1.0)
      (`|ExecutionSequence`
        (:`then_0`
          (`/Engine/EditorBlueprintResources/StandardMacros.DoOnce` false
            (:`Completed`
              (`SplineComponent.AddSplinePoint` _mainspline (`SplineComponent.GetLocationAtSplinePoint` _mainspline _returnvalue_2 "Local") "Local" true)
              (`SplineComponent.SetLocationAtSplinePoint` _mainspline (- _returnvalue_2 2) (`SplineComponent.GetLocationAtDistanceAlongSpline` _mainspline (* (`SplineComponent.GetDistanceAlongSplineAtSplinePoint` _mainspline _returnvalue_2) 0.5) "Local") "Local" true)
              (`self.AddSplineMeshComponent` 0))))
        (:`then_1`
          (for _index (range _returnvalue) :!label _label
            (bind _returnvalue_4 (+ _index 1))
            (`SplineComponent.SetLocationAtSplinePoint` _mainspline_2 _returnvalue_4 (+ (`SplineComponent.GetLocationAtSplinePoint` _mainspline_2 _returnvalue_4 "Local") (`KismetMathLibrary.MakeVector` (`KismetMathLibrary.RandomFloatInRange` _returnvalue_3 _growingrandomxz) (`KismetMathLibrary.RandomFloatInRange` _returnvalue_3 _growingrandomxz) (`self.HeightToGrow`))) "Local" true)
            (if (<= _index (- _returnvalue 2))
              (bind (_location _tangent) (`SplineComponent.GetLocationAndTangentAtSplinePoint` _mainspline_2 _index "Local"))
              (bind (_location_2 _tangent_2) (`SplineComponent.GetLocationAndTangentAtSplinePoint` _mainspline_2 _returnvalue_4 "Local"))
              (`SplineMeshComponent.SetStartAndEnd` (`|GetArrayItem` (`self.set`) _index) _location _tangent _location_2 _tangent_2 true)))
          (if (`self.Head_0`)
            (`SceneComponent.K2_SetRelativeTransform` (`self.HeadRef`) (`KismetMathLibrary.MakeTransform` (.location (`SplineComponent.GetTransformAtSplinePoint` (`self.MainSpline`) _returnvalue "Local" false))) false false))))
      (else
        (goto _label)))))

(fn `AddSplineMeshComponent`
  (params (NewParam :type Integer) (NewParam1 :type Integer))
  (bind _returnvalue (`AddComponent|NODE_AddSplineMeshComponent-2`))
  (`StaticMeshComponent.SetStaticMesh` _returnvalue (`self.Mesh`))
  (`KismetArrayLibrary.Array_Add` (`self.set`) _returnvalue)
  (`KismetSystemLibrary.PrintString` (`KismetSystemLibrary.GetDisplayName` _returnvalue))
  (`SceneComponent.K2_AttachToComponent` _returnvalue (`self.MainSpline`) "None" "SnapToTarget" "SnapToTarget" "KeepRelative" true))

(fn `UserConstructionScript`
  (locals (NumberOfSplinePoints :type Integer))
  (bind _mainspline (`self.MainSpline`))
  (bind _returnvalue (`SplineComponent.GetNumberOfSplinePoints` (`self.MainSpline`)))
  (if (`self.SpawnRoot`)
    (bind _returnvalue_2 (`AddComponent|NODE_AddStaticMeshComponent-1` :`RelativeTransform` (`KismetMathLibrary.MakeTransform` (+ (.location (`SplineComponent.GetTransformAtSplinePoint` (`self.MainSpline`) 0 "Local" false)) (`self.RootMeshOffset`)))))
    (`StaticMeshComponent.SetStaticMesh` _returnvalue_2 (`self.RootMesh`)))
  (set `local.NumberOfSplinePoints` _returnvalue)
  (for _index (range (+ (- _returnvalue (`KismetMathLibrary.SelectInt` 1 2 (`self.Head_0`))) 1))
    (if (and (== (- (`local.NumberOfSplinePoints`) 1) _index) (`self.Head_0`))
      (bind _returnvalue_3 (`AddComponent|NODE_AddStaticMeshComponent-0` :`RelativeTransform` (`KismetMathLibrary.MakeTransform` (.location (`SplineComponent.GetTransformAtSplinePoint` (`self.MainSpline`) _index "Local" false)))))
      (`StaticMeshComponent.SetStaticMesh` _returnvalue_3 (`self.Head`))
      (set `self.HeadRef` _returnvalue_3)
      (else
        (bind _returnvalue_4 (`AddComponent|NODE_AddSplineMeshComponent-1`))
        (`KismetArrayLibrary.Array_Add` (`self.set`) _returnvalue_4)
        (`StaticMeshComponent.SetStaticMesh` _returnvalue_4 (`self.Mesh`))
        (`SceneComponent.K2_AttachToComponent` _returnvalue_4 (`self.MainSpline`) "None" "KeepRelative" "KeepRelative" "KeepRelative" true)
        (bind (_location _tangent) (`SplineComponent.GetLocationAndTangentAtSplinePoint` _mainspline _index "Local"))
        (bind (_location_2 _tangent_2) (`SplineComponent.GetLocationAndTangentAtSplinePoint` _mainspline (+ _index 1) "Local"))
        (`SplineMeshComponent.SetStartAndEnd` _returnvalue_4 _location _tangent _location_2 _tangent_2 true)))))