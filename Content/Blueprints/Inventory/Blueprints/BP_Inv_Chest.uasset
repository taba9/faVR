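; Inventory chest Blueprint that the player can interact with to open or close an inventory UI.
; Interact plays the chest animation once on the skeletal mesh, then checks InventoryOpen to decide whether to close or open the UI.
; The opened UI is stored so its spawned inventory actor can be passed to the close call.
; BeginPlay, overlap and Tick events are unused.
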(event `/Game/Blueprints/InteractionInterface.Interact`
  (`SkeletalMeshComponent.PlayAnimation` (`self.SkeletalMesh`) "/Game/Blueprints/Inventory/Mesh/chest_Anim.chest_Anim" false)
  (if (`self.InventoryOpen?`)
    (`self.CloseInventoryUI` (stale _spawnedinvactor))
    (else
      (bind _spawnedinvactor (`self.OpenInventoryUI`)))))

(fn `UserConstructionScript`
  (`parent.UserConstructionScript`))