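; Inventory display actor that shows the referenced inventory's items as spinning miniature 3D actors laid out in a grid.
; On BeginPlay, GenerateSlots builds centered local Y/Z positions from the slot count and slots per row.
; PopulateSlots then spawns each valid item class scaled down at its slot, disables physics and attaches it to the root.
; Tick rotates every spawned item, while GetItemClass and GetItemData are empty stubs.
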(event `self.ReceiveBeginPlay`
  (set `self.MaxSlot` (`KismetMathLibrary.Conv_IntToDouble` (`/Game/Blueprints/Inventory/Blueprints/BP_Inv_container_master.MaxSlots` (`self.InvRef`))))
  (bind (_invpositiongrid _finish_) (`self.GenerateSlots`))
  (if _finish_
    (`self.PopulateSlots`)))

(event `self.ReceiveActorBeginOverlap`
  (params (OtherActor :type "Actor Object Reference")))

(event `self.ReceiveTick`
  (params (DeltaSeconds :type "Float (single-precision)"))
  (for _array_element (`self.SpawnedActors`)
    (`self.K2_AddActorLocalRotation` _array_element (`KismetMathLibrary.MakeRotator` 0.0 (* DeltaSeconds (`self.RotationSpeed`))) false false)))

(fn `GenerateSlots`
  (returns (InvPositionGrid :type "Array of Vector Structure") (`Finish?` :type Boolean))
  (bind _returnvalue (/ (`self.MaxSlot`) (`self.MaxSlotsPerRow`)))
  (bind _returnvalue_2 (/ _returnvalue 2.0))
  (bind _returnvalue_3 (/ (/ (`self.MaxSlot`) _returnvalue) 2.0))
  (for _index (range (+ (* (`KismetMathLibrary.FTrunc` _returnvalue_2) -1) 1) (+ (`KismetMathLibrary.Round` _returnvalue_2) 1))
    (for _index_2 (range (* (`KismetMathLibrary.FTrunc` _returnvalue_3) -1) (+ (`KismetMathLibrary.FTrunc` _returnvalue_3) 1))
      (`KismetArrayLibrary.Array_Add` (`self.InvSlotPosition`) (`KismetMathLibrary.MakeVector` 0.0 (* _index 30.0) (* _index_2 30.0)))))
  (return (`self.InvSlotPosition`) true))

(fn `GetItemClass`
  (returns (ItemClass :type "/Game/Blueprints/Inventory/Blueprints/S_Inventory_slot Structure"))
  (return))

(fn `GetItemData`
  (returns (`Item Data` :type "/Game/Blueprints/Inventory/Blueprints/S_Item_Info Structure"))
  (return))

(fn `PopulateSlots`
  (returns (`Finish?` :type Boolean))
  (for (_array_element _array_index) (`/Game/Blueprints/Inventory/Blueprints/BP_Inv_container_master.Inventory` (`self.InvRef`))
    (if (`KismetSystemLibrary.IsValidClass` (break `/Game/Blueprints/Inventory/Blueprints/S_Inventory_slot` _array_element))
      (bind _returnvalue (`|SpawnActorFromClass` (break `/Game/Blueprints/Inventory/Blueprints/S_Inventory_slot` _array_element) (`KismetMathLibrary.MakeTransform` (`|GetArrayItem` (`self.InvSlotPosition`) _array_index) (struct) (0.1 0.1 0.1)) "Undefined" "OverrideRootScale"))
      (`PrimitiveComponent.SetSimulatePhysics` (`/Game/Blueprints/Inventory/Blueprints/BP_Item_Master.StaticMesh` _returnvalue) false)
      (`KismetArrayLibrary.Array_Add` (`self.SpawnedActors`) _returnvalue)
      (`self.K2_AttachToComponent` _returnvalue (`self.DefaultSceneRoot`) "None" "KeepRelative" "KeepRelative" "KeepRelative" true)))
  (return true))

(fn `UserConstructionScript`)