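; Master VR inventory actor that stores item classes and amounts in a fixed array of MaxSlots.
; A child placement volume receives a reference to it and supplies item classes through GetItemInput.
; AddItem fills stacks or empty slots, recursively splitting overflow, while RemoveItem rebuilds the array by re-adding its contents.
; Interact toggles a UI handler spawned above the actor and yawed toward the player's camera; overlap-based pickup is disconnected.
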(event `self.ReceiveBeginPlay`
  ;[1 1 1] Set Array to MaxSlots in Inventory
  (`KismetArrayLibrary.Array_Resize` (`self.Inventory`) (`self.MaxSlots`)))

(event `self.ReceiveActorBeginOverlap`
  (params (OtherActor :type "Actor Object Reference")))

(event `self.ReceiveActorEndOverlap`
  (params (OtherActor :type "Actor Object Reference")))

(event `/Game/Blueprints/Inventory/Blueprints/Interfaces/Inv_data_interface.GetItemInput`
  ;[1 1 1] Receive Item input from placementVolume
  (`self.AddItem` (`/Game/Blueprints/BP_PlacementVolume_Master.ItemClass` (cast `/Game/Blueprints/BP_PlacementVolume_Master` (`ChildActorComponent.ChildActor` (`self.BP_inv_input`)) :!pure true))))

(event `/Game/Blueprints/InteractionInterface.Interact`
  (if (`self.InventoryOpen?`)
    (`self.CloseInventoryUI` (stale _spawnedinvactor))
    (else
      (bind _spawnedinvactor (`self.OpenInventoryUI`)))))

(fn `AddItem`
  (params (ItemClass :type "/Game/Blueprints/ItemSystem/Blueprints/BP_Item_Master Class Reference") (Amount :type Integer))
  (returns (`Item added ?` :type Boolean))
  (locals (localClass :type "/Game/Blueprints/ItemSystem/Blueprints/BP_Item_Master Class Reference") (localAmount :type Integer) (FoundIndex :type Integer))
  (bind _returnvalue (+ (`.amount_6_FD1203994A4B89A16E2CA6A4492A079A` (break `/Game/Blueprints/Inventory/Blueprints/Structures/S_Inventory_slot` (`|GetArrayItem` (`self.Inventory`) (`local.FoundIndex`)))) (`local.localAmount`)))
  (set `local.localClass` ItemClass)
  (set `local.localAmount` Amount)
  ;[1 1 1] Check if Item can be stacked
  (if (`.Stackable?_36_4F23189742A89CA049118E8246595A6F` (break `/Game/Blueprints/ItemSystem/Blueprints/Structures/S_Item_Info` (defaults `/Game/Blueprints/Inventory/Blueprints/BP_Inv_master` ItemClass)))
    ;[1 1 1] Search for free Stack in Inventory
    (bind (_found_free_stack_ _index) (`self.SearchFreeStack` (`local.localClass`)))
    (if _found_free_stack_
      ;[1 1 1] Add Items to a free Stack - is there more than MaxStackSize Items get splitted and added to another Slot
      (set `local.FoundIndex` _index)
      (if (> _returnvalue (`self.MaxStackSize`))
        (set `local.localAmount` (- _returnvalue (`self.MaxStackSize`)))
        (`KismetArrayLibrary.Array_Set` (`self.Inventory`) (`local.FoundIndex`) (make `/Game/Blueprints/Inventory/Blueprints/Structures/S_Inventory_slot` (`local.localClass`) (`self.MaxStackSize`)))
        (`self.AddItem` (`local.localClass`) (`local.localAmount`))
        (return false)
        (else
          (`KismetArrayLibrary.Array_Set` (`self.Inventory`) (`local.FoundIndex`) (make `/Game/Blueprints/Inventory/Blueprints/Structures/S_Inventory_slot` (`local.localClass`) _returnvalue))))
      (else
        ;[1 1 1] No free stack found - Add Item to a new Slot - Items more than MaxStackSize get splitted and added to another Slot
        (bind (_index_2 _foundslot_) (`self.SearchEmptySlot`))
        (if _foundslot_
          (bind _output_get (set `local.FoundIndex` _index_2))
          (if (> (`local.localAmount`) (`self.MaxStackSize`))
            (`KismetArrayLibrary.Array_Set` (`self.Inventory`) _output_get (make `/Game/Blueprints/Inventory/Blueprints/Structures/S_Inventory_slot` (`local.localClass`) (`self.MaxStackSize`)))
            (`self.AddItem` (`local.localClass`) (- (`local.localAmount`) (`self.MaxStackSize`)))
            (return true)
            (else
              (`KismetArrayLibrary.Array_Set` (`self.Inventory`) (`local.FoundIndex`) (make `/Game/Blueprints/Inventory/Blueprints/Structures/S_Inventory_slot` (`local.localClass`) (`local.localAmount`)))
              (return true)))
          (else
            (return false)))))
    (else
      ;[1 1 1] Search for Empty Slot if Item cant be stacked and Add Item to Inventory
      (bind (_index_3 _foundslot__2) (`self.SearchEmptySlot`))
      (if _foundslot__2
        ;;[1 1 1] If more then 1 Item that cant be Stacked add to another Slot
        (bind _output_get_2 (set `local.FoundIndex` _index_3))
        (if (> (`local.localAmount`) 1)
          (`KismetArrayLibrary.Array_Set` (`self.Inventory`) _output_get_2 (make `/Game/Blueprints/Inventory/Blueprints/Structures/S_Inventory_slot` (`local.localClass`)))
          (`self.AddItem` (`local.localClass`) (- (`local.localAmount`) 1))
          (return false)
          (else
            (`KismetArrayLibrary.Array_Set` (`self.Inventory`) _output_get_2 (make `/Game/Blueprints/Inventory/Blueprints/Structures/S_Inventory_slot` (`local.localClass`) 0))
            (return true)))
        (else
          (return false))))))

(fn `CloseInventoryUI`
  (params (InventoryRef :type "/Game/Blueprints/Inventory/Blueprints/UI/BP_Inv_UI_Handler Object Reference"))
  (if (`self.InventoryOpen?`)
    (bind _exit_ui (`/Game/Blueprints/Inventory/Blueprints/UI/BP_Inv_UI_Handler.CloseUI` InventoryRef))
    (if _exit_ui
      (set `self.InventoryOpen?` false)
      (`self.K2_DestroyActor` InventoryRef))))

(fn `GetItemClass`
  (returns (ItemClass :type "/Game/Blueprints/Inventory/Blueprints/Structures/S_Inventory_slot Structure"))
  (return))

(fn `GetItemData`
  (returns (`Item Data` :type "/Game/Blueprints/ItemSystem/Blueprints/Structures/S_Item_Info Structure"))
  (return))

(fn `GetItemInfoFromIndex`
  (params (Index :type Integer))
  (returns (`Empty Slot?` :type Boolean) (ItemInfo :type "/Game/Blueprints/ItemSystem/Blueprints/Structures/S_Item_Info Structure") (Amount :type Integer))
  (bind (_itemclass _amount) (break `/Game/Blueprints/Inventory/Blueprints/Structures/S_Inventory_slot` (`|GetArrayItem` (`self.Inventory`) Index)))
  (if (`KismetSystemLibrary.IsValidClass` _itemclass)
    (return false (defaults `/Game/Blueprints/Inventory/Blueprints/BP_Inv_master` _itemclass) _amount)
    (else
      (return true (struct) 0))))

(fn `GetOverlapItemClass`
  (params (`Actor Hit` :type "Actor Object Reference"))
  (returns (ItemClass :type "/Game/Blueprints/ItemSystem/Blueprints/BP_Item_Master Class Reference") (amount :type Integer) (`IsValid?` :type Boolean) (ItemActor :type "Actor Object Reference"))
  (locals (localClass :type "/Game/Blueprints/ItemSystem/Blueprints/BP_Item_Master Class Reference") (localAmount :type Integer) (localBool :type Boolean) (localActor :type "Actor Object Reference"))
  ;[1 1 1] Check if player hands put the item in inventory and than add it when valid to inventory
  (if (== (`GameplayStatics.GetObjectClass` `Actor Hit`) "/Game/Blueprints/BP_MotionController.BP_MotionController_C")
    (bind _asbp_motion_controller (cast `/Game/Blueprints/BP_MotionController` `Actor Hit`))
    (bind _attachedactor (`/Game/Blueprints/BP_MotionController.AttachedActor` _asbp_motion_controller))
    (if (`KismetMathLibrary.ClassIsChildOf` (`GameplayStatics.GetObjectClass` _attachedactor) "/Game/Blueprints/ItemSystem/Blueprints/BP_Item_Master.BP_Item_Master_C")
      (bind _output_get (set `local.localActor` _attachedactor))
      (set `/Game/Blueprints/BP_MotionController.AttachedActor` null _asbp_motion_controller)
      (bind _itemclass (message `/Game/Blueprints/Inventory/Blueprints/Interfaces/Inv_data_interface.GetItemClass` _output_get))
      (set `local.localClass` (break `/Game/Blueprints/Inventory/Blueprints/Structures/S_Inventory_slot` _itemclass))
      (set `local.localAmount` (`.amount_6_FD1203994A4B89A16E2CA6A4492A079A` (break `/Game/Blueprints/Inventory/Blueprints/Structures/S_Inventory_slot` _itemclass)))
      (set `local.localBool` true)
      (return (`local.localClass`) (`local.localAmount`) (`local.localBool`) (`local.localActor`)))
    (else
      ;[1 1 1] Check Item is valid than add to inventory (without hand actor)
      (if (`KismetMathLibrary.ClassIsChildOf` (`GameplayStatics.GetObjectClass` `Actor Hit`) "/Game/Blueprints/ItemSystem/Blueprints/BP_Item_Master.BP_Item_Master_C")
        (bind _output_get_2 (set `local.localActor` `Actor Hit`))
        (bind _itemclass_2 (message `/Game/Blueprints/Inventory/Blueprints/Interfaces/Inv_data_interface.GetItemClass` _output_get_2))
        (set `local.localClass` (break `/Game/Blueprints/Inventory/Blueprints/Structures/S_Inventory_slot` _itemclass_2))
        (set `local.localAmount` (`.amount_6_FD1203994A4B89A16E2CA6A4492A079A` (break `/Game/Blueprints/Inventory/Blueprints/Structures/S_Inventory_slot` _itemclass_2)))
        (set `local.localBool` true)
        (return (`local.localClass`) (`local.localAmount`) (`local.localBool`) (`local.localActor`))))))

(fn `IsEmpty?`
  (params (Index :type Integer))
  (returns (`Empty?` :type Boolean))
  (return (not (`KismetSystemLibrary.IsValidClass` (`.ItemClass_7_DD0C549643319F90FE0F06A625CAF820` (break `/Game/Blueprints/Inventory/Blueprints/Structures/S_Inventory_slot` (`|GetArrayItem` (`self.Inventory`) Index)))))))

(fn `OpenInventoryUI`
  (returns (SpawnedInvActor :type "/Game/Blueprints/Inventory/Blueprints/UI/BP_Inv_UI_Handler Object Reference") (`Open?` :type Boolean))
  ;[1 1 1] New spawn code at Inventory position
  (bind _returnvalue (`|SpawnActorFromClass` "/Game/Blueprints/Inventory/Blueprints/UI/BP_Inv_UI_Handler.BP_Inv_UI_Handler_C" (`KismetMathLibrary.MakeTransform` (`KismetMathLibrary.MakeVector` (.x (`self.K2_GetActorLocation` self)) (.y (`self.K2_GetActorLocation` self)) (+ (.z (`self.K2_GetActorLocation` self)) 20.0)) (`KismetMathLibrary.MakeRotator` 0.0 35.0 (- (.yaw (`SceneComponent.K2_GetComponentRotation` (`/Game/Blueprints/MotionControllerPawn.Camera` (cast `/Game/Blueprints/MotionControllerPawn` (`GameplayStatics.GetPlayerPawn` 0) :!pure true)))) 180.0))) "Undefined" "OverrideRootScale" null self))
  (bind _output_get (set `self.InventoryOpen?` true))
  (return _returnvalue _output_get))

(fn `RemoveItem`
  (params (Index :type Integer) (Amount :type Integer))
  (returns (`Success?` :type Boolean))
  (locals (localClass :type "/Game/Blueprints/ItemSystem/Blueprints/BP_Item_Master Class Reference") (localAmount :type Integer) (localIndex :type Integer))
  (set `local.localIndex` Index)
  (set `local.localAmount` Amount)
  (`KismetArrayLibrary.Array_Set` (`self.Inventory`) (`local.localIndex`) (make `/Game/Blueprints/Inventory/Blueprints/Structures/S_Inventory_slot` null 0))
  (bind _finish (`self.UpdateInventory`))
  (if _finish
    (return true)))

(fn `SearchEmptySlot`
  (returns (Index :type Integer) (`FoundSlot?` :type Boolean))
  (locals (`localSucess?` :type Boolean :default true) (localIndex :type Integer))
  (for (_array_element _array_index) (`self.Inventory`)
    (if (not (`KismetSystemLibrary.IsValidClass` (`.ItemClass_7_DD0C549643319F90FE0F06A625CAF820` (break `/Game/Blueprints/Inventory/Blueprints/Structures/S_Inventory_slot` _array_element))))
      (set `local.localSucess?` true)
      (set `local.localIndex` _array_index)
      (break)))
  (return (`local.localIndex`) (`local.localSucess?`)))

(fn `SearchFreeStack`
  (params (ItemClass :type "/Game/Blueprints/ItemSystem/Blueprints/BP_Item_Master Class Reference"))
  (returns (`found free stack?` :type Boolean) (Index :type Integer))
  (locals (localIndex :type Integer) (loacalbool :type Boolean))
  (for (_array_element _array_index) (`self.Inventory`)
    (bind (_itemclass _amount) (break `/Game/Blueprints/Inventory/Blueprints/Structures/S_Inventory_slot` _array_element))
    (if (`KismetSystemLibrary.IsValidClass` _itemclass)
      (if (and (== _itemclass ItemClass) (<= _amount (`self.MaxStackSize`)))
        (set `local.loacalbool` true)
        (set `local.localIndex` _array_index)
        (break))))
  (return (`local.loacalbool`) (`local.localIndex`)))

(fn `UpdateInventory`
  (returns (Finish :type Boolean))
  (locals (localInventory :type "Array of /Game/Blueprints/Inventory/Blueprints/Structures/S_Inventory_slot Structure"))
  (bind _inventory (`self.Inventory`))
  (set `local.localInventory` _inventory)
  (`KismetArrayLibrary.Array_Clear` _inventory)
  (`KismetArrayLibrary.Array_Resize` _inventory (`self.MaxSlots`))
  (for _array_element (`local.localInventory`)
    (if (`KismetSystemLibrary.IsValidClass` (break `/Game/Blueprints/Inventory/Blueprints/Structures/S_Inventory_slot` _array_element))
      (`self.AddItem` (break `/Game/Blueprints/Inventory/Blueprints/Structures/S_Inventory_slot` _array_element) (`.amount_6_FD1203994A4B89A16E2CA6A4492A079A` (break `/Game/Blueprints/Inventory/Blueprints/Structures/S_Inventory_slot` _array_element)))))
  (return true))

(fn `UserConstructionScript`
  (set `/Game/Blueprints/BP_PlacementVolume_Master.InvRef` self (cast `/Game/Blueprints/BP_PlacementVolume_Master` (`ChildActorComponent.ChildActor` (`self.BP_inv_input`)) :!pure true)))