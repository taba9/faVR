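; BP_Inventory_pouch_test is a test inventory pouch actor that stores items brought into it by a motion controller.
; When a BP_MotionController overlaps it, the pouch passes that controller's attached actor to AddItem.
; Items implementing Inventory_interface_test supply their entry through AddItemMessage, which joins the Inventory array before the actor is destroyed.
; Other actors only print a failure message.
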(event `self.ReceiveActorBeginOverlap`
  (params (OtherActor :type "Actor Object Reference"))
  (bind _asbp_motion_controller (cast `/Game/Blueprints/BP_MotionController` OtherActor))
  (`self.AddItem` (`/Game/Blueprints/BP_MotionController.AttachedActor` _asbp_motion_controller)))

(fn `AddItem`
  (params (Actor :type "Actor Object Reference"))
  (if (`KismetSystemLibrary.DoesImplementInterface` Actor "/Game/Blueprints/Inventory/Blueprints/Inventory_interface_test.Inventory_interface_test_C")
    (bind _item_data (message `/Game/Blueprints/Inventory/Blueprints/Inventory_interface_test.AddItem` Actor))
    (`KismetArrayLibrary.Array_Add` (`self.Inventory`) _item_data)
    (`self.K2_DestroyActor` Actor)
    (else
      (`KismetSystemLibrary.PrintString` (`KismetStringLibrary.BuildString_Object` "" "Failed to insert" Actor)))))

(fn `UserConstructionScript`)