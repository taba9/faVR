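; BP_Item_Master is the item blueprint for the inventory system, holding item data, an amount and a picked-up state.
; The IsPickedUp? event stores the new state and, if the item is in the inventory, has the inventory UI pull it out of the GUI.
; Getter functions return the item's data and its class paired with its amount.
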(event `/Game/Blueprints/InteractionInterface.IsPickedUp?`
  (params (`IsPickedUp?` :type Boolean))
  (set `self.IsCurrentlyPickedUp?` `IsPickedUp?`)
  (if (`self.IsInInventoryItem?`)
    (`/Game/Blueprints/Inventory/Blueprints/Interfaces/Inv_data_interface.PullFromInventoryGUI` (`self.InventoryUiRef`) self)))

(fn `GetItemClass`
  (returns (ItemClass :type "/Game/Blueprints/Inventory/Blueprints/Structures/S_Inventory_slot Structure"))
  (return (make `/Game/Blueprints/Inventory/Blueprints/Structures/S_Inventory_slot` (`GameplayStatics.GetObjectClass` self) (`self.Amount`))))

(fn `GetItemData`
  (returns (`Item Data` :type "/Game/Blueprints/Inventory/Blueprints/Structures/S_Item_Info Structure"))
  (return (`self.Item_Data`)))

(fn `UserConstructionScript`)