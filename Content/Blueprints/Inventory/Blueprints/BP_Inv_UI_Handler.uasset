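; Actor that acts as a 3D inventory UI, showing the items of the referenced inventory as spinning miniature actors.
; On BeginPlay it builds a centered grid of slot positions, then spawns, scales and attaches each item with physics off, and Tick rotates them.
; Pulling an item out restores its scale, removes it from the inventory and rebuilds the display after a short delay.
; CloseUI destroys the miniatures and the handler.
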(event `self.ReceiveBeginPlay`
  (set `self.MaxSlot` (`KismetMathLibrary.Conv_IntToDouble` (`/Game/Blueprints/Inventory/Blueprints/BP_Inv_master.MaxSlots` (`self.InvRef`))))
  (bind (_invpositiongrid _finish_) (`self.GenerateSlots`))
  (if _finish_
    (`self.PopulateSlots`)))

(event `self.ReceiveActorBeginOverlap`
  (params (OtherActor :type "Actor Object Reference")))

(event `self.ReceiveTick`
  (params (DeltaSeconds :type "Float (single-precision)"))
  (if (`self.AnimateUISlots`)
    (for _array_element (`self.SpawnedActors`)
      (`self.K2_AddActorLocalRotation` _array_element (`KismetMathLibrary.MakeRotator` 0.0 (* DeltaSeconds (`self.RotationSpeed`))) false false))))

(event `/Game/Blueprints/Inventory/Blueprints/Interfaces/Inv_data_interface.PullFromInventoryGUI`
  (params (ItemRef :type "/Game/Blueprints/Inventory/Blueprints/BP_Item_Master Object Reference"))
  (`self.PullOutItem` ItemRef)
  (`KismetSystemLibrary.Delay` 0.3)
  (`self.UpdateItemSlots`))

(fn `CloseUI`
  (if (`/Game/Blueprints/Inventory/Blueprints/BP_Inv_master.InventoryOpen?` (`self.InvRef`))
    (for _array_element (`self.SpawnedActors`)
      (`self.K2_DestroyActor` _array_element))
    (`KismetArrayLibrary.Array_Clear` (`self.SpawnedActors`))
    (set `/Game/Blueprints/Inventory/Blueprints/BP_Inv_master.InventoryOpen?` false (`self.InvRef`))
    (`self.K2_DestroyActor`)))

(fn `GenerateSlots`
  (returns (InvPositionGrid :type "Array of Vector Structure") (`Finish?` :type Boolean))
  (bind _returnvalue (/ (`self.MaxSlot`) (`self.MaxSlotsPerRow`)))
  (bind _returnvalue_2 (/ _returnvalue 2.0))
  (bind _returnvalue_3 (/ (/ (`self.MaxSlot`) _returnvalue) 2.0))
  (for _index (range (+ (* (`KismetMathLibrary.FTrunc` _returnvalue_2) -1) 1) (+ (`KismetMathLibrary.Round` _returnvalue_2) 1))
    (for _index_2 (range (* (`KismetMathLibrary.FTrunc` _returnvalue_3) -1) (+ (`KismetMathLibrary.FTrunc` _returnvalue_3) 1))
      (`KismetArrayLibrary.Array_Add` (`self.InvSlotPosition`) (`KismetMathLibrary.MakeVector` 0.0 (* _index 20.0) (* _index_2 20.0)))))
  (set `self.AnimateUISlots` true)
  (return (`self.InvSlotPosition`) true))

(fn `GetItemClass`
  (returns (ItemClass :type "/Game/Blueprints/Inventory/Blueprints/Structures/S_Inventory_slot Structure"))
  (return))

(fn `GetItemData`
  (returns (`Item Data` :type "/Game/Blueprints/Inventory/Blueprints/Structures/S_Item_Info Structure"))
  (return))

(fn `PopulateSlots`
  (returns (`Finish?` :type Boolean))
  (for (_array_element _array_index) (`/Game/Blueprints/Inventory/Blueprints/BP_Inv_master.Inventory` (`self.InvRef`))
    (if (`KismetSystemLibrary.IsValidClass` (break `/Game/Blueprints/Inventory/Blueprints/Structures/S_Inventory_slot` _array_element))
      (bind _returnvalue (`|SpawnActorFromClass` (break `/Game/Blueprints/Inventory/Blueprints/Structures/S_Inventory_slot` _array_element) (`KismetMathLibrary.MakeTransform` (`|GetArrayItem` (`self.InvSlotPosition`) _array_index) (struct) (0.1 0.1 0.1)) "Undefined" "OverrideRootScale"))
      (bind (_item_data_name _item_data_description _item_data_weight _item_data_itemtype _item_data_buyprice _item_data_sellprice _item_data_stackable_ _item_data_useable_ _item_data_miniaturesize) (break `/Game/Blueprints/Inventory/Blueprints/Structures/S_Item_Info` (`/Game/Blueprints/Inventory/Blueprints/BP_Item_Master.Item_Data` _returnvalue)))
      (`self.SetActorScale3D` _returnvalue (`KismetMathLibrary.MakeVector` _item_data_miniaturesize _item_data_miniaturesize _item_data_miniaturesize))
      (set `/Game/Blueprints/Inventory/Blueprints/BP_Item_Master.IsInInventoryItem?` true _returnvalue)
      (set `/Game/Blueprints/Inventory/Blueprints/BP_Item_Master.InventoryUiRef` self _returnvalue)
      (`PrimitiveComponent.SetSimulatePhysics` (`/Game/Blueprints/Inventory/Blueprints/BP_Item_Master.StaticMesh` _returnvalue) false)
      (`KismetArrayLibrary.Array_Add` (`self.SpawnedActors`) _returnvalue)
      (`self.K2_AttachToComponent` _returnvalue (`self.DefaultSceneRoot`) "None" "KeepRelative" "KeepRelative" "KeepRelative" true)
      (set `self.AnimateUISlots` true)))
  (return true))

(fn `PullOutItem`
  (params (ItemRef :type "/Game/Blueprints/Inventory/Blueprints/BP_Item_Master Object Reference"))
  (bind _spawnedactors (`self.SpawnedActors`))
  (for (_array_element _array_index) _spawnedactors
    (if (== _array_element ItemRef)
      (`KismetArrayLibrary.Array_RemoveItem` _spawnedactors ItemRef)
      (`self.K2_SetActorRotation` :`self` ItemRef)
      (set `/Game/Blueprints/Inventory/Blueprints/BP_Item_Master.IsInInventoryItem?` false ItemRef)
      (`self.SetActorScale3D` ItemRef (1.0 1.0 1.0))
      (`/Game/Blueprints/Inventory/Blueprints/BP_Inv_master.RemoveItem` (`self.InvRef`) _array_index (`/Game/Blueprints/Inventory/Blueprints/BP_Item_Master.Amount` ItemRef)))))

(fn `UpdateItemSlots`
  (bind _spawnedactors (`self.SpawnedActors`))
  (set `self.AnimateUISlots` false)
  (for _array_element _spawnedactors
    (`self.K2_DestroyActor` _array_element))
  (`KismetArrayLibrary.Array_Clear` _spawnedactors)
  (`self.PopulateSlots`))

(fn `UserConstructionScript`)