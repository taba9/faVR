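; Base VR inventory container that stores overlapping item actors in a fixed-size slot array and destroys each one when its add reports success.
; AddItem fills matching stacks or empty slots, recursing to split overflow beyond MaxStackSize and to spread non-stackable items.
; A motion controller overlap spawns a BP_Inv_Spawn_Handler in front of the player's camera.
; Ending that overlap destroys its spawned actors and all handlers.
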(event `self.ReceiveBeginPlay`
  ;[1 1 1] Set Array to MaxSlots in Inventory
  (`KismetArrayLibrary.Array_Resize` (`self.Inventory`) (`self.MaxSlots`)))

(event `self.ReceiveActorBeginOverlap`
  (params (OtherActor :type "Actor Object Reference"))
  (if (`KismetMathLibrary.ClassIsChildOf` (`GameplayStatics.GetObjectClass` OtherActor) "/Game/Blueprints/BP_MotionController.BP_MotionController_C")
    (bind _spawnedinvactor (`self.OpenInventory`))
    (else
      (bind (_itemclass _amount _isvalid_ _itemactor) (`self.GetOverlapItemClass` OtherActor))
      (if _isvalid_
        (bind _item_added__ (`self.AddItem` _itemclass _amount))
        (if _item_added__
          (`self.K2_DestroyActor` _itemactor))))))

(event `self.ReceiveActorEndOverlap`
  (params (OtherActor :type "Actor Object Reference"))
  (if (`KismetMathLibrary.ClassIsChildOf` (`GameplayStatics.GetObjectClass` OtherActor) "/Game/Blueprints/BP_MotionController.BP_MotionController_C")
    (`self.CloseInventory` (stale `self.ReceiveActorBeginOverlap` _spawnedinvactor))))

(fn `AddItem`
  (params (ItemClass :type "/Game/Blueprints/Inventory/Blueprints/BP_Item_Master Class Reference") (Amount :type Integer))
  (returns (`Item added ?` :type Boolean))
  (locals (localClass :type "/Game/Blueprints/Inventory/Blueprints/BP_Item_Master Class Reference") (localAmount :type Integer) (FoundIndex :type Integer))
  (bind _returnvalue (+ (`.amount_6_FD1203994A4B89A16E2CA6A4492A079A` (break `/Game/Blueprints/Inventory/Blueprints/S_Inventory_slot` (`|GetArrayItem` (`self.Inventory`) (`local.FoundIndex`)))) (`local.localAmount`)))
  (set `local.localClass` ItemClass)
  (set `local.localAmount` Amount)
  ;[1 1 1] Check if Item can be stacked
  (if (`.Stackable?_36_4F23189742A89CA049118E8246595A6F` (break `/Game/Blueprints/Inventory/Blueprints/S_Item_Info` (defaults `/Game/Blueprints/Inventory/Blueprints/BP_Inv_container_master` ItemClass)))
    ;[1 1 1] Search for free Stack in Inventory
    (bind (_found_free_stack_ _index) (`self.SearchFreeStack` (`local.localClass`)))
    (if _found_free_stack_
      ;[1 1 1] Add Items to a free Stack - is there more than MaxStackSize Items get splitted and added to another Slot
      (set `local.FoundIndex` _index)
      (if (> _returnvalue (`self.MaxStackSize`))
        (set `local.localAmount` (- _returnvalue (`self.MaxStackSize`)))
        (`KismetArrayLibrary.Array_Set` (`self.Inventory`) (`local.FoundIndex`) (make `/Game/Blueprints/Inventory/Blueprints/S_Inventory_slot` (`local.localClass`) (`self.MaxStackSize`)))
        (`self.AddItem` (`local.localClass`) (`local.localAmount`))
        (return true)
        (else
          (`KismetArrayLibrary.Array_Set` (`self.Inventory`) (`local.FoundIndex`) (make `/Game/Blueprints/Inventory/Blueprints/S_Inventory_slot` (`local.localClass`) _returnvalue))))
      (else
        ;[1 1 1] No free stack found - Add Item to a new Slot - Items more than MaxStackSize get splitted and added to another Slot
        (bind (_index_2 _foundslot_) (`self.SearchEmptySlot`))
        (if _foundslot_
          (bind _output_get (set `local.FoundIndex` _index_2))
          (if (> (`local.localAmount`) (`self.MaxStackSize`))
            (`KismetArrayLibrary.Array_Set` (`self.Inventory`) _output_get (make `/Game/Blueprints/Inventory/Blueprints/S_Inventory_slot` (`local.localClass`) (`self.MaxStackSize`)))
            (`self.AddItem` (`local.localClass`) (- (`local.localAmount`) (`self.MaxStackSize`)))
            (return true)
            (else
              (`KismetArrayLibrary.Array_Set` (`self.Inventory`) (`local.FoundIndex`) (make `/Game/Blueprints/Inventory/Blueprints/S_Inventory_slot` (`local.localClass`) (`local.localAmount`)))
              (return true)))
          (else
            (return false)))))
    (else
      ;[1 1 1] Search for Empty Slot if Item cant be stacked and Add Item to Inventory
      (bind (_index_3 _foundslot__2) (`self.SearchEmptySlot`))
      (if _foundslot__2
        (bind _output_get_2 (set `local.FoundIndex` _index_3))
        (`KismetArrayLibrary.Array_Set` (`self.Inventory`) _output_get_2 (make `/Game/Blueprints/Inventory/Blueprints/S_Inventory_slot` (`local.localClass`)))
        ;;[1 1 1] If more then 1 Item that cant be Stacked add to another Slot
        (if (> (`local.localAmount`) 1)
          (`self.AddItem` (`local.localClass`) (- (`local.localAmount`) 1))
          (return true))
        (else
          (return false))))))

(fn `CloseInventory`
  (params (InventoryRef :type "/Game/Blueprints/Inventory/Blueprints/BP_Inv_Spawn_Handler Object Reference"))
  (if (`self.InventoryOpen?`)
    (for _array_element (`/Game/Blueprints/Inventory/Blueprints/BP_Inv_Spawn_Handler.SpawnedActors` InventoryRef)
      (`self.K2_DestroyActor` _array_element))
    (bind _outactors (`GameplayStatics.GetAllActorsOfClass` "/Game/Blueprints/Inventory/Blueprints/BP_Inv_Spawn_Handler.BP_Inv_Spawn_Handler_C"))
    (for _array_element_2 _outactors
      (`self.K2_DestroyActor` _array_element_2))
    (set `self.InventoryOpen?` false)))

(fn `GetItemInfoFromIndex`
  (params (Index :type Integer))
  (returns (`Empty Slot?` :type Boolean) (ItemInfo :type "/Game/Blueprints/Inventory/Blueprints/S_Item_Info Structure") (Amount :type Integer))
  (bind (_itemclass _amount) (break `/Game/Blueprints/Inventory/Blueprints/S_Inventory_slot` (`|GetArrayItem` (`self.Inventory`) Index)))
  (if (`KismetSystemLibrary.IsValidClass` _itemclass)
    (return false (defaults `/Game/Blueprints/Inventory/Blueprints/BP_Inv_container_master` _itemclass) _amount)
    (else
      (return true (struct) 0))))

(fn `GetOverlapItemClass`
  (params (`Actor Hit` :type "Actor Object Reference"))
  (returns (ItemClass :type "/Game/Blueprints/Inventory/Blueprints/BP_Item_Master Class Reference") (amount :type Integer) (`IsValid?` :type Boolean) (ItemActor :type "Actor Object Reference"))
  (locals (localClass :type "/Game/Blueprints/Inventory/Blueprints/BP_Item_Master Class Reference") (localAmount :type Integer) (localBool :type Boolean) (localActor :type "Actor Object Reference"))
  ;[1 1 1] Check if player hands put the item in inventory and than add it when valid to inventory
  (if (== (`GameplayStatics.GetObjectClass` `Actor Hit`) "/Game/Blueprints/Backup/BP_MotionController.BP_MotionController_C")
    (bind _asbp_motion_controller (cast `/Game/Blueprints/BP_MotionController` `Actor Hit`))
    (bind _attachedactor (`/Game/Blueprints/BP_MotionController.AttachedActor` _asbp_motion_controller))
    (if (`KismetSystemLibrary.DoesImplementInterface` _attachedactor "/Game/Blueprints/Inventory/Blueprints/Inventory_interface.Inventory_interface_C")
      (bind _output_get (set `local.localActor` _attachedactor))
      (bind _itemclass (message `/Game/Blueprints/Inventory/Blueprints/Inventory_interface.GetItemClass` _output_get))
      (set `local.localClass` (break `/Game/Blueprints/Inventory/Blueprints/S_Inventory_slot` _itemclass))
      (set `local.localAmount` (`.amount_6_FD1203994A4B89A16E2CA6A4492A079A` (break `/Game/Blueprints/Inventory/Blueprints/S_Inventory_slot` _itemclass)))
      (set `local.localBool` true)
      (return (`local.localClass`) (`local.localAmount`) (`local.localBool`) (`local.localActor`)))
    (else
      ;[1 1 1] Check Item is valid than add to inventory (without hand actor)
      (if (`KismetMathLibrary.ClassIsChildOf` (`GameplayStatics.GetObjectClass` `Actor Hit`) "/Game/Blueprints/Inventory/Blueprints/BP_Item_Master.BP_Item_Master_C")
        (bind _output_get_2 (set `local.localActor` `Actor Hit`))
        (bind _itemclass_2 (message `/Game/Blueprints/Inventory/Blueprints/Inventory_interface.GetItemClass` _output_get_2))
        (set `local.localClass` (break `/Game/Blueprints/Inventory/Blueprints/S_Inventory_slot` _itemclass_2))
        (set `local.localAmount` (`.amount_6_FD1203994A4B89A16E2CA6A4492A079A` (break `/Game/Blueprints/Inventory/Blueprints/S_Inventory_slot` _itemclass_2)))
        (set `local.localBool` true)
        (return (`local.localClass`) (`local.localAmount`) (`local.localBool`) (`local.localActor`))))))

(fn `IsEmpty?`
  (params (Index :type Integer))
  (returns (`Empty?` :type Boolean))
  (return (not (`KismetSystemLibrary.IsValidClass` (`.ItemClass_3_DD0C549643319F90FE0F06A625CAF820` (break `/Game/Blueprints/Inventory/Blueprints/S_Inventory_slot` (`|GetArrayItem` (`self.Inventory`) Index)))))))

(fn `OpenInventory`
  (returns (SpawnedInvActor :type "/Game/Blueprints/Inventory/Blueprints/BP_Inv_Spawn_Handler Object Reference") (`Open?` :type Boolean))
  (bind _camera (`/Game/Blueprints/MotionControllerPawn.Camera` (cast `/Game/Blueprints/MotionControllerPawn` (`GameplayStatics.GetPlayerPawn` 0) :!pure true)))
  (if (not (`self.InventoryOpen?`))
    (bind _returnvalue (`|SpawnActorFromClass` "/Game/Blueprints/Inventory/Blueprints/BP_Inv_Spawn_Handler.BP_Inv_Spawn_Handler_C" (`KismetMathLibrary.MakeTransform` (+ (`SceneComponent.K2_GetComponentLocation` _camera) (* (`SceneComponent.GetForwardVector` _camera) 100.0)) (`KismetMathLibrary.MakeRotator` 90.0 (.pitch (`SceneComponent.K2_GetComponentRotation` _camera)) (.yaw (`SceneComponent.K2_GetComponentRotation` _camera))) (1.0 1.0 1.0)) "Undefined" "OverrideRootScale" null self))
    (bind _output_get (set `self.InventoryOpen?` true))
    (return _returnvalue _output_get)))

(fn `SearchEmptySlot`
  (returns (Index :type Integer) (`FoundSlot?` :type Boolean))
  (locals (`localSucess?` :type Boolean :default true) (localIndex :type Integer))
  (for (_array_element _array_index) (`self.Inventory`)
    (if (not (`KismetSystemLibrary.IsValidClass` (`.ItemClass_3_DD0C549643319F90FE0F06A625CAF820` (break `/Game/Blueprints/Inventory/Blueprints/S_Inventory_slot` _array_element))))
      (set `local.localSucess?` true)
      (set `local.localIndex` _array_index)
      (break)))
  (return (`local.localIndex`) (`local.localSucess?`)))

(fn `SearchFreeStack`
  (params (ItemClass :type "/Game/Blueprints/Inventory/Blueprints/BP_Item_Master Class Reference"))
  (returns (`found free stack?` :type Boolean) (Index :type Integer))
  (locals (localIndex :type Integer) (loacalbool :type Boolean))
  (for (_array_element _array_index) (`self.Inventory`)
    (bind (_itemclass _amount) (break `/Game/Blueprints/Inventory/Blueprints/S_Inventory_slot` _array_element))
    (if (`KismetSystemLibrary.IsValidClass` _itemclass)
      (if (and (== _itemclass ItemClass) (<= _amount (`self.MaxStackSize`)))
        (set `local.loacalbool` true)
        (set `local.localIndex` _array_index)
        (break))))
  (return (`local.loacalbool`) (`local.localIndex`)))

(fn `UserConstructionScript`)