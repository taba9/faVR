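; Placement volume actor that snaps overlapping actors into place, such as props dropped into a slot.
; The construction script adds a box, sphere or capsule collision component chosen by CollisionBoxType, with configurable offset, rotation and size.
; On overlap, an actor with no attach parent is snapped and welded to that shape, keeping world scale, and its static mesh physics simulation is switched off.
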(event `self.ReceiveBeginPlay`)

(event `self.ReceiveActorBeginOverlap`
  (params (OtherActor :type "Actor Object Reference"))
  (if (== (`self.GetAttachParentActor` OtherActor) null)
    (switch `/Game/Blueprints/PlacementVolumeEnum` (`self.CollisionBoxType`)
      (:`NewEnumerator0`
        (`self.K2_AttachToComponent` OtherActor (`self.BoxCollision`) "None" "SnapToTarget" "SnapToTarget" "KeepWorld" true))
      (:`NewEnumerator1`
        (`self.K2_AttachToComponent` OtherActor (`self.SphereCollision`) "None" "SnapToTarget" "SnapToTarget" "KeepWorld" true))
      (:`NewEnumerator2`
        (`self.K2_AttachToComponent` OtherActor (`self.CapsuleCollision`) "None" "SnapToTarget" "SnapToTarget" "KeepWorld" true)))
    (`PrimitiveComponent.SetSimulatePhysics` (`self.GetComponentByClass` OtherActor "/Script/Engine.StaticMeshComponent") false)))

(fn `UserConstructionScript`
  (bind (_x _y) (`KismetMathLibrary.BreakVector2D` (`self.CapsuleHalfHeight&Radius`)))
  (bind _returnvalue (`ActorComponent.GetOwner` (`self.Scene`)))
  (bind _returnvalue_2 (`KismetMathLibrary.MakeTransform` (`self.Offset`) (`self.Rotation`)))
  (switch `/Game/Blueprints/PlacementVolumeEnum` (`self.CollisionBoxType`)
    (:`NewEnumerator0`
      (bind _returnvalue_3 (`AddComponent|NODE_AddBoxComponent-1` :`self` _returnvalue :`RelativeTransform` _returnvalue_2))
      (`BoxComponent.SetBoxExtent` _returnvalue_3 (`self.BoxExtent`) true)
      (set `self.BoxCollision` _returnvalue_3))
    (:`NewEnumerator1`
      (bind _returnvalue_4 (`AddComponent|NODE_AddSphereComponent-0` :`self` _returnvalue :`RelativeTransform` _returnvalue_2))
      (`SphereComponent.SetSphereRadius` _returnvalue_4 (`self.SphereRadius`) true)
      (set `self.SphereCollision` _returnvalue_4))
    (:`NewEnumerator2`
      (bind _returnvalue_5 (`AddComponent|NODE_AddCapsuleComponent-0` :`self` _returnvalue :`RelativeTransform` _returnvalue_2))
      (`CapsuleComponent.SetCapsuleSize` _returnvalue_5 _y _x true)
      (set `self.CapsuleCollision` _returnvalue_5))))