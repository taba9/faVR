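; Master placement volume that holds a single BP_Item_Master item of a matching type, or feeds items into an inventory.
; The construction script builds a configurable box, sphere or capsule collider.
; Overlaps (optional) or the Add event supply actors; unparented interactable items attach with physics off, offset to align their "Grip" socket.
; Inventory mode instead records the item class, destroys the actor and calls InvRef's GetItemInput.
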(event `self.ReceiveActorBeginOverlap`
  (params (OtherActor :type "Actor Object Reference"))
  (bind _actortoattach (`self.ActorToAttach`))
  (bind _returnvalue (`self.GetComponentByClass` _actortoattach "/Script/Engine.StaticMeshComponent"))
  (if (`self.AllowNonAttachedActors?`)
    (set `self.ActorToAttach` OtherActor)
    (if (`self.IsInventoryPlacement?`) :!label _label
      (if (`KismetMathLibrary.ClassIsChildOf` (`GameplayStatics.GetObjectClass` (`self.ActorToAttach`)) "/Game/Blueprints/ItemSystem/Blueprints/BP_Item_Master.BP_Item_Master_C")
        (bind _itemclass (`self.GetClassToInput` (`self.ActorToAttach`)))
        (bind _output_get (set `self.ItemClass` _itemclass))
        (`KismetSystemLibrary.PrintString` (`KismetSystemLibrary.GetClassDisplayName` _output_get))
        (`/Game/Blueprints/Inventory/Blueprints/Interfaces/Inv_data_interface.GetItemInput` (`self.InvRef`)))
      (else
        (bind _still_attached_ (`self.ItemStillAttached?`))
        (if _still_attached_
          _
          (elif (`KismetMathLibrary.ClassIsChildOf` (`GameplayStatics.GetObjectClass` (`self.ActorToAttach`)) "/Game/Blueprints/ItemSystem/Blueprints/BP_Item_Master.BP_Item_Master_C")
            (bind _asbp_item_master (cast `/Game/Blueprints/ItemSystem/Blueprints/BP_Item_Master` (`self.ActorToAttach`)))
            (if (`|EnumEquality` (`.ItemType_51_0E9547FC41FF6F79B1E8FDA24B2057F8` (break `/Game/Blueprints/ItemSystem/Blueprints/Structures/S_Item_Info` (`/Game/Blueprints/ItemSystem/Blueprints/BP_Item_Master.Item_Data` _asbp_item_master))) (`self.ItemType`))
              (if (`self.ObjectStored`)
                _
                (elif (and (== (`self.GetAttachParentActor` _actortoattach) null) (`KismetSystemLibrary.DoesImplementInterface` _actortoattach "/Game/Blueprints/InteractionInterface.InteractionInterface_C"))
                  (bind _attachedactor (`self.AttachItemToPlacementVolume` _returnvalue (`self.ActorToAttach`)))
                  (set `self.AttachedActor` _attachedactor)
                  (set `self.ObjectStored` true)
                  (`self.SetActorLocationOffset` _returnvalue))))))))))

(event `Add`
  (params (Actor :type "Actor Object Reference"))
  (set `self.ActorToAttach` Actor)
  (goto _label))

(fn `AttachItemToPlacementVolume`
  (params (Component :type "PrimitiveComponent Object Reference") (Actor :type "Actor Object Reference"))
  (returns (AttachedActor :type "Actor Object Reference"))
  (switch `/Game/Blueprints/PlacementVolumeEnum` (`self.CollisionBoxType`)
    (:`NewEnumerator0`
      (`self.K2_AttachToComponent` Actor (`self.BoxCollision`) "None" (`self.LocationAttachment`) (`self.RotationAttachment`) "KeepWorld" true))
    (:`NewEnumerator1`
      (`self.K2_AttachToComponent` Actor (`self.SphereCollision`) "None" (`self.LocationAttachment`) (`self.RotationAttachment`) "KeepWorld" true))
    (:`NewEnumerator2`
      (`self.K2_AttachToComponent` Actor (`self.CapsuleCollision`) "None" (`self.LocationAttachment`) (`self.RotationAttachment`) "KeepWorld" true)))
  (`PrimitiveComponent.SetSimulatePhysics` Component false)
  (return Actor))

(fn `GetClassToInput`
  (params (InputActor :type "Actor Object Reference"))
  (returns (ItemClass :type "/Game/Blueprints/ItemSystem/Blueprints/BP_Item_Master Class Reference"))
  (locals (localClass :type "/Game/Blueprints/ItemSystem/Blueprints/BP_Item_Master Class Reference"))
  (bind _attachedactor (`self.AttachedActor`))
  (bind _output_get (set `self.AttachedActor` InputActor))
  (bind _returnvalue (`GameplayStatics.GetObjectClass` _output_get))
  (if (`KismetSystemLibrary.IsValidClass` _returnvalue)
    (if (`KismetMathLibrary.ClassIsChildOf` _returnvalue "/Game/Blueprints/ItemSystem/Blueprints/BP_Item_Master.BP_Item_Master_C")
      (bind _itemclass (`/Game/Blueprints/ItemSystem/Blueprints/BP_Item_Master.GetItemClass` (cast `/Game/Blueprints/ItemSystem/Blueprints/BP_Item_Master` _attachedactor :!pure true)))
      (set `local.localClass` (break `/Game/Blueprints/Inventory/Blueprints/Structures/S_Inventory_slot` _itemclass))
      (`self.K2_DestroyActor` _attachedactor)
      (set `self.AttachedActor` null)
      (return (`local.localClass`)))))

(fn `GetItemClass`
  (returns (ItemClass :type "/Game/Blueprints/Inventory/Blueprints/Structures/S_Inventory_slot Structure"))
  (return))

(fn `GetItemData`
  (returns (`Item Data` :type "/Game/Blueprints/ItemSystem/Blueprints/Structures/S_Item_Info Structure"))
  (return))

(fn `ItemStillAttached?`
  (returns (`Still attached?` :type Boolean))
  (bind _attachedactor (`self.AttachedActor`))
  (`/Engine/EditorBlueprintResources/StandardMacros.IsValid` _attachedactor
    (:`Is Valid`
      (if (== (`self.GetAttachParentActor` _attachedactor) (`self.NewVar_0`))
        (return true)
        (else
          _)))
    (:`Is Not Valid`
      _))
  (set `self.ObjectStored` false)
  (set `self.AttachedActor` null)
  (return false))

(fn `SetActorLocationOffset`
  (params (Component :type "PrimitiveComponent Object Reference"))
  (bind _attachedactor (`self.AttachedActor`))
  (bind _returnvalue (`KismetMathLibrary.NegateRotator` (`KismetMathLibrary.NormalizedDeltaRotator` (.rotation (`SceneComponent.GetSocketTransform` Component "Grip" "RTS_Actor")))))
  (`self.K2_SetActorRelativeRotation` _attachedactor _returnvalue false false)
  (`self.K2_SetActorRelativeLocation` _attachedactor (+ (`KismetMathLibrary.GreaterGreater_VectorRotator` (`KismetMathLibrary.NegateVector` (.location (`SceneComponent.GetSocketTransform` Component "Grip" "RTS_Actor"))) _returnvalue) (`self.ActorAttachOffset`)) false false))

(fn `UserConstructionScript`
  (bind (_x _y) (`KismetMathLibrary.BreakVector2D` (`self.CapsuleHalfHeight&Radius`)))
  (bind _returnvalue (`ActorComponent.GetOwner` (`self.Scene`)))
  (bind _returnvalue_2 (`KismetMathLibrary.MakeTransform` (`self.Offset`) (`self.Rotation`)))
  (set `self.NewVar_0` self)
  (switch `/Game/Blueprints/PlacementVolumeEnum` (`self.CollisionBoxType`)
    (:`NewEnumerator0`
      (bind _returnvalue_3 (`AddComponent|NODE_AddBoxComponent-1` :`self` _returnvalue :`RelativeTransform` _returnvalue_2))
      (`BoxComponent.SetBoxExtent` _returnvalue_3 (`self.BoxExtent`) false)
      (set `self.BoxCollision` _returnvalue_3))
    (:`NewEnumerator1`
      (bind _returnvalue_4 (`AddComponent|NODE_AddSphereComponent-0` :`self` _returnvalue :`RelativeTransform` _returnvalue_2))
      (`SphereComponent.SetSphereRadius` _returnvalue_4 (`self.SphereRadius`) false)
      (set `self.SphereCollision` _returnvalue_4))
    (:`NewEnumerator2`
      (bind _returnvalue_5 (`AddComponent|NODE_AddCapsuleComponent-0` :`self` _returnvalue :`RelativeTransform` _returnvalue_2))
      (`CapsuleComponent.SetCapsuleSize` _returnvalue_5 _y _x false)
      (set `self.CapsuleCollision` _returnvalue_5))))