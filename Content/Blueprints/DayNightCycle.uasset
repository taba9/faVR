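; Day/night cycle Blueprint that positions the sun from latitude, time of day and day of year.
; BeginPlay offsets the time drives by CurrentTime; the construction script sets initial sun rotation.
; Timeline update logic, with no wired trigger shown, uses solar-declination math for day length and sun angles.
; It also switches sun and skylight intensity, updates the sky sphere and advances the day count.
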(event `self.ReceiveBeginPlay`
  (bind _currenttime (`self.CurrentTime`))
  (`/Engine/EditorBlueprintResources/StandardMacros.DoOnce` false
    (:`Completed`
      (set `self.YawDrive` (+ (* _currenttime (`self.EquatorFlip`)) (`self.YawDrive`)))
      (set `self.PitchDrive` (+ _currenttime (`self.PitchDrive`))))))

(fn `UserConstructionScript`
  (`self.SetActorRotation` (`self.Lightsource`) (`KismetMathLibrary.MakeRotator` 0.0 (`self.pitch`) (`self.Yaw`)))
  (`/Engine/EngineSky/BP_Sky_Sphere.UpdateSunDirection` (`self.SkySphere`)))